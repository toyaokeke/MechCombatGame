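; Spawner actor that creates AI spider enemies at its own location in the mech combat game.
; SpawnExplosive spawns a Spider_Bomb and SpawnTurret spawns a Spider_Turret, each increasing the ThirdPersonGameMode's active and total created bot counters.
; The event graph is empty, so both functions run only when called from elsewhere.
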(fn `SpawnExplosive`
  (`AIBlueprintHelperLibrary.SpawnAIFromClass` "/Game/ThirdPersonBP/Blueprints/Spider_Bomb.Spider_Bomb_C" null (`self.K2_GetActorLocation`) (struct) false null)
  (bind _asthird_person_game_mode (cast `/Game/ThirdPersonBP/Blueprints/ThirdPersonGameMode` (`GameplayStatics.GetGameMode`)))
  (`/Engine/EditorBlueprintResources/StandardMacros.IncrementInt` (`/Game/ThirdPersonBP/Blueprints/ThirdPersonGameMode.NumberOfBots` _asthird_person_game_mode)
    (:`  `
      (`/Engine/EditorBlueprintResources/StandardMacros.IncrementInt` (`/Game/ThirdPersonBP/Blueprints/ThirdPersonGameMode.NumberOfBotsCreated` _asthird_person_game_mode)))))

(fn `SpawnTurret`
  (`AIBlueprintHelperLibrary.SpawnAIFromClass` "/Game/ThirdPersonBP/Blueprints/Spider_Turret.Spider_Turret_C" null (`self.K2_GetActorLocation`) (struct) false null)
  (bind _asthird_person_game_mode (cast `/Game/ThirdPersonBP/Blueprints/ThirdPersonGameMode` (`GameplayStatics.GetGameMode`)))
  (`/Engine/EditorBlueprintResources/StandardMacros.IncrementInt` (`/Game/ThirdPersonBP/Blueprints/ThirdPersonGameMode.NumberOfBots` _asthird_person_game_mode)
    (:`  `
      (`/Engine/EditorBlueprintResources/StandardMacros.IncrementInt` (`/Game/ThirdPersonBP/Blueprints/ThirdPersonGameMode.NumberOfBotsCreated` _asthird_person_game_mode)))))

(fn `UserConstructionScript`)