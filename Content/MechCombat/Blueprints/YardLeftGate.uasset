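; YardLeftGate is a gate actor that swings open when a ThirdPersonCharacter enters its box and closes when one leaves.
; Separate open and close timelines drive the mesh's yaw, each behind a DoOnce that resets on timeline updates.
; Projectile overlaps on the mesh spawn explosions; wall damage and destruction logic follows, but casts that same overlapping actor to YardWalls, so it only runs if that cast also succeeds.
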(event `self.Box.OnComponentBeginOverlap`
  (params (OverlappedComponent :type "PrimitiveComponent Object Reference") (OtherActor :type "Actor Object Reference") (OtherComp :type "PrimitiveComponent Object Reference") (OtherBodyIndex :type Integer) (bFromSweep :type Boolean) (SweepResult :type "HitResult Structure (by ref)"))
  ;[1 1 1] Open Gate
  (cast `/Game/ThirdPersonBP/Blueprints/ThirdPersonCharacter` OtherActor)
  (`/Engine/EditorBlueprintResources/StandardMacros.DoOnce` false :!label _label
    (:`Completed`
      (bind (_direction _newtrack_0) (`Timeline|OpenGate` :!via `PlayFromStart`)
        (:`Update`
          (`SceneComponent.K2_SetRelativeRotation` (`self.StaticMesh`) (`KismetMathLibrary.MakeRotator` 0.0 0.0 _newtrack_0) false false)
          (goto _label :!via `Reset`))))))

(event `self.Box.OnComponentEndOverlap`
  (params (OverlappedComponent :type "PrimitiveComponent Object Reference") (OtherActor :type "Actor Object Reference") (OtherComp :type "PrimitiveComponent Object Reference") (OtherBodyIndex :type Integer))
  ;[1 1 1] Close Gate
  (cast `/Game/ThirdPersonBP/Blueprints/ThirdPersonCharacter` OtherActor)
  (`/Engine/EditorBlueprintResources/StandardMacros.DoOnce` false :!label _label_2
    (:`Completed`
      (bind (_direction _newtrack_0) (`Timeline|CloseGate` :!via `PlayFromStart`)
        (:`Update`
          (`SceneComponent.K2_SetRelativeRotation` (`self.StaticMesh`) (`KismetMathLibrary.MakeRotator` 0.0 0.0 _newtrack_0) false false)
          (goto _label_2 :!via `Reset`))))))

(event `self.StaticMesh.OnComponentBeginOverlap`
  (params (OverlappedComponent :type "PrimitiveComponent Object Reference") (OtherActor :type "Actor Object Reference") (OtherComp :type "PrimitiveComponent Object Reference") (OtherBodyIndex :type Integer) (bFromSweep :type Boolean) (SweepResult :type "HitResult Structure (by ref)"))
  ;[1 1 1] Projectile Handler
  (bind _asprojectile (cast `/Game/MechCombat/Blueprints/Projectile` OtherActor))
  (`GameplayStatics.SpawnEmitterAtLocation` "/Game/StarterContent/Particles/P_Explosion.P_Explosion" (`self.K2_GetActorLocation` _asprojectile))
  (bind _asyard_walls (cast `/Game/MechCombat/Blueprints/YardWalls` OtherActor))
  (bind _output_get (set `/Game/MechCombat/Blueprints/YardWalls.Health` (- (`/Game/MechCombat/Blueprints/YardWalls.Health` _asyard_walls) (/ (`/Game/MechCombat/Blueprints/Projectile.TurretDamage` _asprojectile) 2.0)) _asyard_walls))
  (if (<= _output_get 0.0)
    (`GameplayStatics.SpawnEmitterAtLocation` "/Game/StarterContent/Particles/P_Explosion.P_Explosion" (`self.K2_GetActorLocation` _asyard_walls) (struct) (10.0 10.0 10.0))
    (`self.K2_DestroyActor` _asprojectile)
    (`self.K2_DestroyActor` _asyard_walls)
    (`self.K2_DestroyActor`)
    (else
      (`self.K2_DestroyActor` _asprojectile))))

(fn `UserConstructionScript`)